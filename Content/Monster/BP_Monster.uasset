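; BP_Monster is an enemy that hunts through a behavior tree and ends the game with a scream the first time the player character overlaps it.
; AI perception updates write the InPerception flag to the blackboard and, on a successful sense, the sensed actor as TargetActor.
; A successful sense also starts an attached chase sound, unless one is already playing, and stores it in the blackboard.
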(event `self.ReceiveBeginPlay`
  (`AIController.RunBehaviorTree` (`AIBlueprintHelperLibrary.GetAIController` self) "/Game/Monster/BT_Monster.BT_Monster"))

(event `self.ReceiveActorBeginOverlap`
  (params (OtherActor :type "Actor Object Reference"))
  (bind _asfirst_person_character (cast `/Game/FirstPersonBP/Blueprints/FirstPersonCharacter` OtherActor))
  (`/Engine/EditorBlueprintResources/StandardMacros.DoOnce` false
    (:`Completed`
      (`/Game/FirstPersonBP/Blueprints/FirstPersonCharacter.Game Over` _asfirst_person_character false)
      (`GameplayStatics.PlaySound2D` "/Game/Sounds/scream_Cue.scream_Cue" 1.0 1.0 0.0 null null))))

(event `self.AIPerception.OnTargetPerceptionUpdated`
  (params (Actor :type "Actor Object Reference") (Stimulus :type "AIStimulus Structure"))
  (`BlackboardComponent.SetValueAsBool` (`AIBlueprintHelperLibrary.GetBlackboard` self) "InPerception" Stimulus_bSuccessfullySensed)
  (if Stimulus_bSuccessfullySensed
    (`|ExecutionSequence`
      (:`then_0`
        (bind _lastsound (`self.LastSound`)
          (:`then`
            (if (not (`AudioComponent.IsPlaying` _lastsound))
              (bind _returnvalue (`GameplayStatics.SpawnSoundAttached` "/Game/Sounds/chase_Cue.chase_Cue" (`self.CapsuleComponent`) "None" (0.0 0.0 0.0) (struct) "KeepRelativeOffset" false 1.0 1.0 0.0 null null :!label _label))
              (bind _output_get (set `self.LastSound` _returnvalue))
              (`BlackboardComponent.SetValueAsObject` (`AIBlueprintHelperLibrary.GetBlackboard` self) "Sound" _output_get)))
          (:`else`
            (goto _label))))
      (:`then_1`
        (`BlackboardComponent.SetValueAsObject` (`AIBlueprintHelperLibrary.GetBlackboard` self) "TargetActor" Actor)))))

(fn `UserConstructionScript`)