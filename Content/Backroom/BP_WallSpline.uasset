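; Wall segment actor for procedural Backroom generation, built from a spline mesh that grows along its local X axis.
; Each Update extends the end until the wall is Dead; SetDead freezes it and destroys walls no longer than MinLength.
; Branching rolls against a length-based probability from the owning BP_SplineGenerator.
; Collision checks box-trace the end point for other walls, filtering out parent-child links.
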(event `Update`
  (bind _splinemesh (`self.SplineMesh`))
  (if (not (`self.Dead`))
    (`SplineMeshComponent.SetEndPosition` _splinemesh (+ (`SplineMeshComponent.GetEndPosition` _splinemesh) (* (1.0 0.0 0.0) (`self.IncrementAmount`))) true)))

(event `SetEndLocation`
  (params (Location :type "Vector Structure"))
  (`SplineMeshComponent.SetEndPosition` (`self.SplineMesh`) (- Location (`self.K2_GetActorLocation`)) true))

(event `Set Length`
  (params (Length :type "Float (double-precision)"))
  (bind (_returnvalue_x _returnvalue_y _returnvalue_z) (`KismetMathLibrary.BreakVector` (`self.K2_GetActorLocation`)))
  (`SplineMeshComponent.SetEndPosition` (`self.SplineMesh`) (`KismetMathLibrary.MakeVector` (+ _returnvalue_x Length) _returnvalue_y _returnvalue_z) true))

(fn `CheckCollision`
  (params (Distance :type "Float (double-precision)") (Parent :type "/Game/Backroom/BP_WallSpline Object Reference"))
  (returns (Collide :type Boolean) (Object :type "/Game/Backroom/BP_WallSpline Object Reference"))
  (bind _loc (`self.GetEnd`))
  (bind _outhits (`KismetSystemLibrary.BoxTraceMultiForObjects` :`Start` _loc :`End` _loc :`HalfSize` (`KismetMathLibrary.Conv_DoubleToVector` Distance) :`ObjectTypes` (`|MakeArray` "ObjectTypeQuery1" :!type "EObjectTypeQuery Enum") :`DrawTime` 1.0))
  (for _array_element _outhits
    (bind _asbp_wall_spline (cast `/Game/Backroom/BP_WallSpline` (`.HitActor` (`GameplayStatics.BreakHitResult` _array_element))))
    (if (and (!= _asbp_wall_spline Parent) (!= self (`/Game/Backroom/BP_WallSpline.Parent` _asbp_wall_spline)) (!= (`self.Parent`) _asbp_wall_spline))
      (return true _asbp_wall_spline)))
  (return false null))

(fn `GetEnd`
  (returns (Loc :type "Vector Structure"))
  (return (`KismetMathLibrary.TransformLocation` (`self.GetTransform`) (`SplineMeshComponent.GetEndPosition` (`self.SplineMesh`)))))

(fn `Set Dead`
  (set `self.Dead` true)
  (if (<= (`KismetMathLibrary.VSize` (- (`self.GetEnd`) (`self.K2_GetActorLocation`))) (`self.Min Length`))
    (`self.K2_DestroyActor`)))

(fn `ShouldBranch`
  (returns (Should :type Boolean))
  (bind _asbp_spline_generator (cast `/Game/Backroom/BP_SplineGenerator` (`self.GetOwner`)))
  (bind _probability (`/Game/Backroom/BP_SplineGenerator.CalculateProbability` _asbp_spline_generator (`KismetMathLibrary.VSize` (- (`self.GetEnd`) (`self.K2_GetActorLocation`))) 1.0))
  (return (and (>= _probability (`KismetMathLibrary.RandomFloat`)) (not (`self.Dead`)))))

(fn `UserConstructionScript`)