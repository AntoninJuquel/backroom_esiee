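; BP_LightSwitch is an interactable switch that controls every BP_LIght sharing its LightIndex.
; On BeginPlay it gathers all BP_LIght actors in the level into an array.
; On Interact it sends InteractMessage to lights with a matching index, then flips IsOn and swaps its Cube material between green and red to show its state.
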(event `self.ReceiveBeginPlay`
  (bind _outactors (`GameplayStatics.GetAllActorsOfClass` "/Game/Interactable/BP_LIght.BP_LIght_C"))
  (for _array_element _outactors
    (`KismetArrayLibrary.Array_Add` (`self.LightsArray`) _array_element)))

(event `/Game/Interactable/I_Interactable.Interact`
  (params (Player :type "/Game/FirstPersonBP/Blueprints/FirstPersonCharacter Object Reference"))
  (bind _cube (`self.Cube`))
  (for _array_element (`self.LightsArray`)
    (if (== (`/Game/Interactable/BP_LIght.LightIndex` _array_element) (`self.LightIndex`))
      (message `/Game/Interactable/I_Interactable.Interact` _array_element null)))
  (bind _output_get (set `self.IsOn` (not (`self.IsOn`))))
  (if _output_get
    (`PrimitiveComponent.SetMaterial` _cube 0 "/Game/Interactable/Green.Green")
    (else
      (`PrimitiveComponent.SetMaterial` _cube 0 "/Game/Interactable/Red.Red"))))

(fn `UserConstructionScript`)