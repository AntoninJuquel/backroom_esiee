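; BP_Locker is an interactable locker that the player can unlock with a key, step into and step out of.
; When locked, Interact asks the player to use a key of a set type; success permanently unlocks it and turns its point light green.
; Entering moves the player to the locker's origin, storing the move's success as PlayerInside.
; Interacting while inside moves the player out in front of the locker.
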(event `/Game/Interactable/I_Interactable.Interact`
  (params (Player :type "/Game/FirstPersonBP/Blueprints/FirstPersonCharacter Object Reference"))
  (if (`self.PlayerInside`)
    (`self.K2_SetActorLocation` Player (+ (`self.K2_GetActorLocation`) (* (`self.GetActorForwardVector`) 200.0)) false false)
    (set `self.PlayerInside` false)
    (elif (`self.Unlocked`)
      (bind (_sweephitresult _returnvalue) (`self.K2_SetActorLocation` Player (`self.K2_GetActorLocation`) false false :!label _label))
      (set `self.PlayerInside` _returnvalue)
      (set `self.Unlocked` true)
      (`LightComponent.SetLightColor` (`self.PointLight`) (struct :`G` 1.0 :`A` 1.0) true)
      (else
        (bind _success (`/Game/FirstPersonBP/Blueprints/FirstPersonCharacter.UseKey` Player "NewEnumerator2"))
        (if _success
          (goto _label))))))

(fn `UserConstructionScript`)