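; BP_LIght is an interactable light that toggles on and off.
; Its Interact event flips the IsOn flag and applies it as the visibility of the SpotLight and PointLight components together.
; The construction script applies the same flag to both components, so the placed light reflects its initial IsOn state.
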(event `/Game/Interactable/I_Interactable.Interact`
  (params (Player :type "/Game/FirstPersonBP/Blueprints/FirstPersonCharacter Object Reference"))
  (bind _output_get (set `self.IsOn` (not (`self.IsOn`))))
  (`SceneComponent.SetVisibility` (`self.SpotLight`) _output_get false)
  (`SceneComponent.SetVisibility` (`self.PointLight`) _output_get false))

(fn `UserConstructionScript`
  (`SceneComponent.SetVisibility` (`self.SpotLight`) (`self.IsOn`) false)
  (`SceneComponent.SetVisibility` (`self.PointLight`) (`self.IsOn`) false))